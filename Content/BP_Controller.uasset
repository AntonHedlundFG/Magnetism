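; BP_Controller is a player controller that lets the player pick magnets with the mouse.
; On BeginPlay it creates the WBP_UI widget, enables game-and-UI input with a visible cursor, and adds the IAC_Main mapping context.
; IA_Select deprojects the mouse position, has MagnetismPhysicsSystem trace that ray against magnet spheres, and passes the result to the UI as the selected magnet.
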(event `self.ReceiveBeginPlay`
  (bind _returnvalue (`|CreateWidget` "/Game/WBP_UI.WBP_UI_C" self))
  (bind _output_get (set `self.InteractUI` _returnvalue))
  (`UserWidget.AddToViewport` _output_get 0)
  (`WidgetBlueprintLibrary.SetInputMode_GameAndUIEx` self _returnvalue)
  (set `self.bShowMouseCursor` true)
  (`EnhancedInputSubsystemInterface.AddMappingContext` (subsystem `EnhancedInputLocalPlayerSubsystem`) "/Game/IAC_Main.IAC_Main" 0 (struct)))

(event `EnhancedInput|/Game/IA_Select`
  (params (ActionValue :type Boolean) (ElapsedSeconds :type "Float (double-precision)") (TriggeredSeconds :type "Float (double-precision)") (InputAction :type "InputAction Object Reference" :default "/Game/IA_Select.IA_Select"))
  (:`Started`
    (`self.SelectHoveredObject`)))

(fn `SelectHoveredObject`
  (bind (_worldlocation _worlddirection) (`self.DeprojectMousePositionToWorld`))
  (`/Game/WBP_UI.SetSelectedMagnet` (`self.InteractUI`) (`MagnetismPhysicsSystem.TraceLineForMagnetSpheres` (subsystem `MagnetismPhysicsSystem`) _worldlocation _worlddirection)))

(fn `UserConstructionScript`)